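; Activateable platform actor that is hidden when activated and shown when deactivated.
; BeginPlay starts it hidden with collision disabled, the same state that Activate applies.
; Deactivate makes it visible and restores collision, so visibility and collision always toggle together.
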(event EventBeginPlay
  (|CallParentFunction)
  (Rendering|SetActorHiddenInGame true)
  (Collision|SetActorEnableCollision false))

(event Collision|EventActorBeginOverlap
  (params (OtherActor :type Actor%20Object%20Reference))
  (|CallParentFunction OtherActor) ; This node is disabled and will not be called.\nDrag off pins to build functionality.
)

(event EventTick
  (params (DeltaSeconds :type Float%20%28single-precision%29))
  (|CallParentFunction DeltaSeconds) ; This node is disabled and will not be called.\nDrag off pins to build functionality.
)

(event EventActivate
  (Rendering|SetActorHiddenInGame true)
  (Collision|SetActorEnableCollision false))

(event EventDeactivate
  (Rendering|SetActorHiddenInGame false)
  (Collision|SetActorEnableCollision true))

(fn ConstructionScript
  (|CallParentFunction))