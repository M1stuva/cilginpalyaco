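; An activateable moving platform that shuttles its Cube back and forth between FirstPos and Pos while activated.
; Activate and Deactivate toggle a flag that gates Tick, which teleports the cube at constant speed without sweeping.
; On nearing the target, it flips IsReversed and swaps targets.
; Direction uses the cube's relative location but movement applies world offsets; the InterpToMovement setup is unconnected.
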(event EventBeginPlay
  (|CallParentFunction)
  (Variables|Default|SetTargetPos (Variables|Default|GetPos)))

(event Collision|EventActorBeginOverlap
  (params (OtherActor :type Actor%20Object%20Reference))
  (|CallParentFunction OtherActor) ; This node is disabled and will not be called.\nDrag off pins to build functionality.
)

(event EventActivate
  (Variables|Default|SetIsActivated true))

(event EventDeactivate
  (Variables|Default|SetIsActivated false))

(event EventTick
  (params (DeltaSeconds :type Float%20%28single-precision%29))
  (bind _cube (Variables|Default|GetCube))
  (bind _targetpos (Variables|Default|GetTargetPos))
  (bind _returnvalue (Transformation|GetRelativeTransform _cube))
  (bind _returnvalue_2 (- _targetpos (.location _returnvalue)))
  (bind _returnvalue_3 (Math|Vector|Normalize _returnvalue_2))
  (if (Variables|Default|GetIsActivated)
    (if (Variables|Default|GetIsReversed)
      (CallFunction|MovetoPosition DeltaSeconds 3e+02 _returnvalue_3)
      (else
        (CallFunction|MovetoPosition DeltaSeconds 3e+02 _returnvalue_3)))
    (CallFunction|CheckifReachedGoal)))

(fn ConstructionScript
  (|CallParentFunction))

(fn MovetoPosition
  (params (deltaSeconds :type Float%20%28double-precision%29) (Velocity :type Float%20%28double-precision%29) (MoveDirection :type Vector))
  (Transformation|AddWorldOffset (Variables|Default|GetCube) (* deltaSeconds Velocity MoveDirection) false true))

(fn CheckifReachedGoal
  (if (< (Math|Vector|Distance(Vector) (.location (Transformation|GetRelativeTransform (Variables|Default|GetCube))) (Variables|Default|GetTargetPos)) 1e+01)
    (bind _output_get (Variables|Default|SetIsReversed (not (Variables|Default|GetIsReversed))))
    (if _output_get
      (Variables|Default|SetTargetPos (Variables|Default|GetFirstPos))
      (else
        (Variables|Default|SetTargetPos (Variables|Default|GetPos))))))